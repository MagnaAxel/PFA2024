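; Player character Blueprint that turns Enhanced Input actions into world-axis movement, jumping and a forward dash launch.
; Move input also calls Rotate, which sets capsule yaw toward the first entry in Threats during combat, or along the input direction otherwise.
; Dash uses LaunchCharacter along the actor's forward vector, adding to current velocity.
; Interact and Attack inputs are empty stubs.
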(event EventBeginPlay)

(event Collision|EventActorBeginOverlap
  (params (OtherActor :type Actor%20Object%20Reference)))

(event EventTick
  (params (DeltaSeconds :type Float%20%28single-precision%29)))

(event Input|EnhancedActionEvents|EnhancedInputActionIA_Move
  (params (ActionValue :type Vector%202D%20Structure) (ElapsedSeconds :type Float%20%28double-precision%29) (TriggeredSeconds :type Float%20%28double-precision%29) (InputAction :type Input%20Action%20Object%20Reference :default "/Game/Dynamic/Blueprints/Characters/Player/Inputs/Actions/IA_Move.IA_Move"))
  (bind (_x _y) (Math|Vector2D|BreakVector2D ActionValue))
  (bind _returnvalue (Math|Vector|MakeVector _x _y 0.0))
  (:Triggered
    (Pawn|Input|AddMovementInput _returnvalue 1.0 false)
    (CallFunction|Rotate _returnvalue)))

(event Input|EnhancedActionEvents|EnhancedInputActionIA_Jump
  (params (ActionValue :type Boolean) (ElapsedSeconds :type Float%20%28double-precision%29) (TriggeredSeconds :type Float%20%28double-precision%29) (InputAction :type Input%20Action%20Object%20Reference :default "/Game/Dynamic/Blueprints/Characters/Player/Inputs/Actions/IA_Jump.IA_Jump"))
  (:Triggered
    (Character|Jump)))

(event Input|EnhancedActionEvents|EnhancedInputActionIA_Dash
  (params (ActionValue :type Boolean) (ElapsedSeconds :type Float%20%28double-precision%29) (TriggeredSeconds :type Float%20%28double-precision%29) (InputAction :type Input%20Action%20Object%20Reference :default "/Game/Dynamic/Blueprints/Characters/Player/Inputs/Actions/IA_Dash.IA_Dash"))
  (:Triggered
    (Character|LaunchCharacter (* (Transformation|GetActorForwardVector self) "1000.000000,1000.000000,0.000000") false false)))

(event Input|EnhancedActionEvents|EnhancedInputActionIA_Interact
  (params (ActionValue :type Boolean) (ElapsedSeconds :type Float%20%28double-precision%29) (TriggeredSeconds :type Float%20%28double-precision%29) (InputAction :type Input%20Action%20Object%20Reference :default "/Game/Dynamic/Blueprints/Characters/Player/Inputs/Actions/IA_Interact.IA_Interact")))

(event Input|EnhancedActionEvents|EnhancedInputActionIA_Attack
  (params (ActionValue :type Boolean) (ElapsedSeconds :type Float%20%28double-precision%29) (TriggeredSeconds :type Float%20%28double-precision%29) (InputAction :type Input%20Action%20Object%20Reference :default "/Game/Dynamic/Blueprints/Characters/Player/Inputs/Actions/IA_Attack.IA_Attack")))

(fn ConstructionScript
  (|CallParentFunction))

(fn Rotate
  (params (Vector :type Vector%20%28by%20ref%29))
  (if (Variables|Default|GetIsInCombat)
    (Transformation|SetWorldRotation (Variables|Default|GetCapsuleComponent) (Math|Rotator|MakeRotator 0.0 0.0 (.yaw (Math|Rotator|FindLookatRotation (Transformation|GetActorLocation) (Transformation|GetActorLocation (Utilities|Array|Get(acopy) (Variables|Default|GetThreats)))))) false false)
    (else
      (Transformation|SetWorldRotation (Variables|Default|GetCapsuleComponent) (Math|Rotator|MakeRotator 0.0 0.0 (Class|KismetAnimationLibrary|CalculateDirection Vector (Math|Rotator|MakeRotator 0.0 0.0 0.0))) false false))))