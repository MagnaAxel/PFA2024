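; PC_Player is the player controller that creates and possesses the player's character when play begins.
; On BeginPlay it asks the game mode for the PlayerStart, spawns PlayerClass at that transform and possesses the new actor.
; It then adds the IM_Player mapping context to the Enhanced Input local player subsystem at base priority.
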(event EventBeginPlay
  (bind _returnvalue (Game|SpawnActorfromClass (Variables|Default|GetPlayerClass) (Transformation|GetActorTransform (Class|GameModeBase|FindPlayerStart (Game|GetGameMode) 0 (Variables|Default|GetPlayerStart))) "Undefined" "MultiplyWithRoot" 0 0))
  (Pawn|Possess self _returnvalue)
  (Input|AddMappingContext (PlayerController|LocalPlayerSubsystems|GetEnhancedInputLocalPlayerSubsystem self) "/Game/Dynamic/Blueprints/Characters/Player/Inputs/Maps/IM_Player.IM_Player" 0 "(bIgnoreAllPressedKeysUntilRelease=True,bForceImmediately=False,bNotifyUserSettings=False)"))

(fn ConstructionScript)