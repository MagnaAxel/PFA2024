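; BP_Item is an interactable pickup actor that places an item into the player's inventory.
; Its construction script looks up the Name row in DT_Item and stores it as Item, printing an error if the row is missing.
; On Interact, it appends Item to the Items array in the player's BPInventory and then destroys itself.
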(event EventInteract
  (params (Player :type BP%20Player%20Object%20Reference))
  (Utilities|Array|Add (.Items (Utilities|Struct|BreakST_Inventory (Variables|/Game/Dynamic/Blueprints/Characters/Inventory/BP_Inventory.BP_Inventory_C|GetInventory (Variables|/Game/Dynamic/Blueprints/Characters/BP_Character.BP_Character_C|GetBP_Inventory Player)))) (Variables|Default|GetItem))
  (Actor|DestroyActor))

(fn ConstructionScript
  (bind _returnvalue (Utilities|GetDataTableRow "/Game/Dynamic/Blueprints/Items/DT_Item.DT_Item" (Variables|Default|GetName))
    (:then
      (Variables|Default|SetItem _returnvalue))
    (:RowNotFound
      (Development|PrintString "Item not found!" true true "(R=1.000000,G=0.000000,B=0.018072,A=1.000000)"))))